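; BP_PuertaArriba is a door actor that opens when a Character enters its trigger box and closes when one leaves.
; BeginPlay caches the relative locations of the door and of a Destino component that marks the open position.
; Overlap begin plays and overlap end reverses a single timeline, which lerps the door between those two locations.
; Exits are not counted, so any Character leaving starts the closing even if another remains inside.
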(event OnComponentBeginOverlap(TriggerBoxCollision)
  (params (OverlappedComponent :type Primitive%20Component%20Object%20Reference) (OtherActor :type Actor%20Object%20Reference) (OtherComp :type Primitive%20Component%20Object%20Reference) (OtherBodyIndex :type Integer) (bFromSweep :type Boolean) (SweepResult :type Hit%20Result%20Structure%20%28by%20ref%29))
  (Utilities|Casting|CastToCharacter OtherActor)
  (bind _newtrack_0 (Timeline|Timeline_0 Play)
    (:Update
      (Transformation|SetRelativeLocation (Variables|Default|GetPuerta) (Math|Vector|Lerp(Vector) (Variables|Default|GetPuertaLocation) (Variables|Default|GetDestinoLocation) _newtrack_0) false false))))

(event OnComponentEndOverlap(TriggerBoxCollision)
  (params (OverlappedComponent :type Primitive%20Component%20Object%20Reference) (OtherActor :type Actor%20Object%20Reference) (OtherComp :type Primitive%20Component%20Object%20Reference) (OtherBodyIndex :type Integer))
  (Utilities|Casting|CastToCharacter OtherActor)
  (bind _newtrack_0 (Timeline|Timeline_0 Reverse)
    (:Update
      (Transformation|SetRelativeLocation (Variables|Default|GetPuerta) (Math|Vector|Lerp(Vector) (Variables|Default|GetPuertaLocation) (Variables|Default|GetDestinoLocation) _newtrack_0) false false))))

(event EventBeginPlay
  (Variables|Default|SetPuertaLocation (Variables|/Script/Engine.SceneComponent|GetRelativeLocation (Variables|Default|GetPuerta)))
  (Variables|Default|SetDestinoLocation (Variables|/Script/Engine.SceneComponent|GetRelativeLocation (Variables|Default|GetDestino))))

(event Collision|EventActorBeginOverlap
  (params (OtherActor :type Actor%20Object%20Reference)))

(event EventTick
  (params (DeltaSeconds :type Float%20%28single-precision%29)))

(fn ConstructionScript)