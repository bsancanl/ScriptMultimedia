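; BP_ItemMoneda is a coin pickup that adds its point value to the player's total score.
; On BeginPlay it caches the ThirdPersonGameMode.
; When a Character overlaps its Box, it adds Puntaje to the game mode's PuntajeTotal, writes the new total directly to the game mode's HUD, then destroys itself.
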(event OnComponentBeginOverlap(Box)
  (params (OverlappedComponent :type Primitive%20Component%20Object%20Reference) (OtherActor :type Actor%20Object%20Reference) (OtherComp :type Primitive%20Component%20Object%20Reference) (OtherBodyIndex :type Integer) (bFromSweep :type Boolean) (SweepResult :type Hit%20Result%20Structure%20%28by%20ref%29))
  (bind _as_third_person_game_mode (Variables|Default|GetAs%20Third%20Person%20Game%20Mode))
  ;[1 1 1] Evaluo si el actor con el que se esta interactuando es un BP del tipo character
  (Utilities|Casting|CastToCharacter OtherActor)
  ;[1 1 1] Acceso a la variable Puntaje Total del BP GameMode para sumarle un el puntaje del item y luego guardar el valor
  (bind _output_get (Variables|/Game/ThirdPersonBP/Blueprints/ThirdPersonGameMode.ThirdPersonGameMode_C|SetPuntajeTotal _as_third_person_game_mode (+ (Variables|/Game/ThirdPersonBP/Blueprints/ThirdPersonGameMode.ThirdPersonGameMode_C|GetPuntajeTotal _as_third_person_game_mode) (Variables|Default|GetPuntaje))))
  ;[1 1 1] Accedo a la interfaz grafica HUD por medio del BP Game Mode para enviar y mostrar el puntaje en pantalla
  (Variables|/Game/ClaseScript/Blueprints/UI/HUD.HUD_C|SetPuntajeValor (Variables|/Game/ThirdPersonBP/Blueprints/ThirdPersonGameMode.ThirdPersonGameMode_C|GetHUD (Variables|Default|GetAs%20Third%20Person%20Game%20Mode)) _output_get)
  (Actor|DestroyActor))

(event EventBeginPlay
  ;[1 1 1] Obtengo la referencia hacia el Game mode para luego castear y guardar el BP ThirdPersonGamemode en una variable
  (bind _asthird_person_game_mode (Utilities|Casting|CastToThirdPersonGameMode (Game|GetGameMode)))
  (Variables|Default|SetAs%20Third%20Person%20Game%20Mode _asthird_person_game_mode))

(event Collision|EventActorBeginOverlap
  (params (OtherActor :type Actor%20Object%20Reference)))

(fn ConstructionScript)