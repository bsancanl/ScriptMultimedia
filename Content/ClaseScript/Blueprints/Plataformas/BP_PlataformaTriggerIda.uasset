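; Moving platform that travels one way ("Ida") when a Character enters its trigger Box.
; BeginPlay stores the relative locations of the Cube and of a Scene component that marks the destination.
; The overlap plays the Movimiento timeline, whose value lerps the Cube between those points without sweep.
; A Loop branch meant for back-and-forth motion is left unconnected and never runs.
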(event OnComponentBeginOverlap(Box)
  (params (OverlappedComponent :type Primitive%20Component%20Object%20Reference) (OtherActor :type Actor%20Object%20Reference) (OtherComp :type Primitive%20Component%20Object%20Reference) (OtherBodyIndex :type Integer) (bFromSweep :type Boolean) (SweepResult :type Hit%20Result%20Structure%20%28by%20ref%29))
  (Utilities|Casting|CastToCharacter OtherActor)
  ;[1 1 1] Se crea un grafica que entregara valores desde 0 a 1 en un tiempo de 5 segundos
  (bind _valores (Timeline|Movimiento Play)
    (:Update
      ;[1 1 1] Con la funcion Lerp (vectores) podemos realizar una transicion entre dos valores vectoriales (AyB) utilizando el parametro (Alpha). Mientras el valor de Alpha se acerque a 0 el resultado sera cercano a la Posicion Inicial, caso contrario si se acerca a 1 el resultado sera cercano a la Posicion Final
      (Transformation|SetRelativeLocation (Variables|Default|GetCube) (Math|Vector|Lerp(Vector) (Variables|Default|GetPosicionRelativaInicial) (Variables|Default|GetPosicionRelativaFinal) _valores) false false))))

(event EventBeginPlay
  ;[1 1 1] Guardamos la posicion relativa inicial del cubo y la posicion realtiva inicial ddel componente Scene (el cual sera la posicion a donde queremos que se mueva la plataforma
  (Variables|Default|SetPosicionRelativaInicial (Variables|/Script/Engine.SceneComponent|GetRelativeLocation (Variables|Default|GetCube)))
  (Variables|Default|SetPosicionRelativaFinal (Variables|/Script/Engine.SceneComponent|GetRelativeLocation (Variables|Default|GetScene))))

(event Collision|EventActorBeginOverlap
  (params (OtherActor :type Actor%20Object%20Reference)))

(event EventTick
  (params (DeltaSeconds :type Float%20%28single-precision%29)))

(fn ConstructionScript)