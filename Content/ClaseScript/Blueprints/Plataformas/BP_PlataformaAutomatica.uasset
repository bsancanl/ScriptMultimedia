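; Automatic moving platform that starts on BeginPlay and shuttles its Cube back and forth between its initial position and a Scene component marking the destination.
; The Movimiento timeline drives a vector Lerp between the two cached relative locations to move the Cube.
; On Finished, the Loop flag alternates between Reversa and Iniciar for endless motion, while Detener stops the timeline.
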(event Custom|Reversa
  ;[1 1 1] Creamos varios eventos para poder manejar las etapas del timeline
  ;[1 1 1] Se crea un grafica que entregara valores desde 0 a 1 en un tiempo de 5 segundos
  (bind _valores (Timeline|Movimiento Reverse)
    (:Update
      ;[1 1 1] Con la funcion Lerp (vectores) podemos realizar una transicion entre dos valores vectoriales (AyB) utilizando el parametro (Alpha). Mientras el valor de Alpha se acerque a 0 el resultado sera cercano a la Posicion Inicial, caso contrario si se acerca a 1 el resultado sera cercano a la Posicion Final
      (Transformation|SetRelativeLocation (Variables|Default|GetCube) (Math|Vector|Lerp(Vector) (Variables|Default|GetPosicionRelativaInicial) (Variables|Default|GetPosicionRelativaFinal) _valores) false false))
    (:Finished
      ;[1 1 1] Con la ayuda del Branch y al colocar TRUE como valor inicial a la variable Loop podremos crear un movimiento infinito de la plataforma
      (if (Variables|Default|GetLoop)
        (Variables|Default|SetLoop false)
        (CallFunction|Reversa)
        (else
          (Variables|Default|SetLoop true)
          (CallFunction|Iniciar))))))

(event Custom|Detener
  ;[1 1 1] Creamos varios eventos para poder manejar las etapas del timeline
  ;[1 1 1] Se crea un grafica que entregara valores desde 0 a 1 en un tiempo de 5 segundos
  (bind _valores (Timeline|Movimiento Stop)
    (:Update
      ;[1 1 1] Con la funcion Lerp (vectores) podemos realizar una transicion entre dos valores vectoriales (AyB) utilizando el parametro (Alpha). Mientras el valor de Alpha se acerque a 0 el resultado sera cercano a la Posicion Inicial, caso contrario si se acerca a 1 el resultado sera cercano a la Posicion Final
      (Transformation|SetRelativeLocation (Variables|Default|GetCube) (Math|Vector|Lerp(Vector) (Variables|Default|GetPosicionRelativaInicial) (Variables|Default|GetPosicionRelativaFinal) _valores) false false))
    (:Finished
      ;[1 1 1] Con la ayuda del Branch y al colocar TRUE como valor inicial a la variable Loop podremos crear un movimiento infinito de la plataforma
      (if (Variables|Default|GetLoop)
        (Variables|Default|SetLoop false)
        (CallFunction|Reversa)
        (else
          (Variables|Default|SetLoop true)
          (CallFunction|Iniciar))))))

(event Custom|Iniciar
  ;[1 1 1] Creamos varios eventos para poder manejar las etapas del timeline
  ;[1 1 1] Se crea un grafica que entregara valores desde 0 a 1 en un tiempo de 5 segundos
  (bind _valores (Timeline|Movimiento Play)
    (:Update
      ;[1 1 1] Con la funcion Lerp (vectores) podemos realizar una transicion entre dos valores vectoriales (AyB) utilizando el parametro (Alpha). Mientras el valor de Alpha se acerque a 0 el resultado sera cercano a la Posicion Inicial, caso contrario si se acerca a 1 el resultado sera cercano a la Posicion Final
      (Transformation|SetRelativeLocation (Variables|Default|GetCube) (Math|Vector|Lerp(Vector) (Variables|Default|GetPosicionRelativaInicial) (Variables|Default|GetPosicionRelativaFinal) _valores) false false))
    (:Finished
      ;[1 1 1] Con la ayuda del Branch y al colocar TRUE como valor inicial a la variable Loop podremos crear un movimiento infinito de la plataforma
      (if (Variables|Default|GetLoop)
        (Variables|Default|SetLoop false)
        (CallFunction|Reversa)
        (else
          (Variables|Default|SetLoop true)
          (CallFunction|Iniciar))))))

(event EventBeginPlay
  ;[1 1 1] Iniciamos la animacion al momento de iniciar el juego, ademas guardamos la posicion relativa inicial del cubo y la posicion realtiva inicial ddel componente Scene (el cual sera la posicion a donde queremos que se mueva la plataforma
  (Variables|Default|SetPosicionRelativaInicial (Variables|/Script/Engine.SceneComponent|GetRelativeLocation (Variables|Default|GetCube)))
  (Variables|Default|SetPosicionRelativaFinal (Variables|/Script/Engine.SceneComponent|GetRelativeLocation (Variables|Default|GetScene)))
  (CallFunction|Iniciar))

(event Collision|EventActorBeginOverlap
  (params (OtherActor :type Actor%20Object%20Reference)))

(event EventTick
  (params (DeltaSeconds :type Float%20%28single-precision%29)))

(fn ConstructionScript)