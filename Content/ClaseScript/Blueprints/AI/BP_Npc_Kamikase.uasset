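; BP_Npc_Kamikase is a kamikaze NPC that chases the player and explodes on reaching them.
; Pawn sensing detects a ThirdPersonCharacter, and a one-time flag stores the reference and blocks retriggering on later sightings.
; AI MoveTo follows that actor, and on success the NPC spawns a scaled explosion particle, plays a sound and destroys itself.
; The explosion applies no damage in this graph, and a failed move has no handling.
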(event OnSeePawn(PawnSensing)
  (params (Pawn :type Pawn%20Object%20Reference))
  ;[1 1 1] Detecta al player la primera vez para guardar la referencia de a quien va a perseguir por el resto del juego, ademas se usa una variable PLAYER DETECTADO para evitar que se vuelva activar la programacion en el evento On See Pawn
  (bind _asthird_person_character (Utilities|Casting|CastToThirdPersonCharacter Pawn))
  (if (not (Variables|Default|GetPlayerDetectado))
    (Variables|Default|SetPlayerDetectado true)
    (Variables|Default|SetAs%20Third%20Person%20Character _asthird_person_character)
    (AI|AIMoveTo self "0, 0, 0" (Variables|Default|GetAs%20Third%20Person%20Character) 5.0 false
      (:OnSuccess
        ;[1 1 1] Se crea una particula P_Explosion en la posicion del enemigo en cuanto alcanza al player
        (Effects|SpawnEmitteratLocation "/Game/StarterContent/Particles/P_Explosion.P_Explosion" (Transformation|GetActorLocation) "0, 0, 0" "5.000000,5.000000,5.000000")
        ;[1 1 1] Se ejecuta una sonido de explosion luego de alcanzar al player
        (Audio|PlaySoundatLocation "/Game/StarterContent/Audio/Explosion02.Explosion02" (Transformation|GetActorLocation) "0, 0, 0" 1.0 1.0 0.0 0 0 0)
        (Actor|DestroyActor)))))

(event EventBeginPlay)

(event Collision|EventActorBeginOverlap
  (params (OtherActor :type Actor%20Object%20Reference)))

(event EventTick
  (params (DeltaSeconds :type Float%20%28single-precision%29)))

(fn ConstructionScript)